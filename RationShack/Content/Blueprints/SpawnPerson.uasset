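; Spawner actor that keeps one randomly chosen person in play at its spawn point.
; On BeginPlay and whenever the SpawnNewPerson event fires, it spawns a random actor class, destroys the previous person and randomizes the new mesh's material.
; It drives the person's Move component, calling NewPerson after each spawn and Stamped when the F key is released.
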(event Custom|SpawnedNewPerson_Event
  (bind _materials (Variables|Components|GetMaterials))
  (bind _actors (Variables|Components|GetActors))
  (bind _returnvalue (Game|SpawnActorfromClass (Utilities|Array|Get(acopy) _actors (Math|Random|RandomInteger (Utilities|Array|Length _actors))) (Variables|Default|GetSpawnPoint) "Undefined" 0 0))
  (Utilities|IsValid (Variables|Default|GetSpawnedPerson)
    (:Is%20Valid
      (Actor|DestroyActor (Variables|Default|GetSpawnedPerson)))
    (:Is%20Not%20Valid
      _))
  (bind _output_get (Variables|Default|SetSpawnedPerson _returnvalue))
  (Default|CallNewPerson (Utilities|Array|Get(acopy) (Actor|GetComponentsByClass (Variables|Default|GetSpawnedPerson) "/Game/Blueprints/Move.Move_C")))
  (Rendering|Material|SetMaterial (Utilities|Array|Get(acopy) (Actor|GetComponentsByClass _output_get "/Script/Engine.MeshComponent")) 0 (Utilities|Array|Get(acopy) _materials (Math|Random|RandomInteger (Utilities|Array|Length _materials)))))

(event EventBeginPlay
  (bind _materials (Variables|Components|GetMaterials))
  (bind _actors (Variables|Components|GetActors))
  (EventDispatchers|BindEventtoSpawnNewPerson (delegate Custom|SpawnedNewPerson_Event))
  (Input|EnableInput (Game|GetPlayerController 0))
  (bind _returnvalue (Game|SpawnActorfromClass (Utilities|Array|Get(acopy) _actors (Math|Random|RandomInteger (Utilities|Array|Length _actors))) (Variables|Default|GetSpawnPoint) "Undefined" 0 0))
  (Utilities|IsValid (Variables|Default|GetSpawnedPerson)
    (:Is%20Valid
      (Actor|DestroyActor (Variables|Default|GetSpawnedPerson)))
    (:Is%20Not%20Valid
      _))
  (bind _output_get (Variables|Default|SetSpawnedPerson _returnvalue))
  (Default|CallNewPerson (Utilities|Array|Get(acopy) (Actor|GetComponentsByClass (Variables|Default|GetSpawnedPerson) "/Game/Blueprints/Move.Move_C")))
  (Rendering|Material|SetMaterial (Utilities|Array|Get(acopy) (Actor|GetComponentsByClass _output_get "/Script/Engine.MeshComponent")) 0 (Utilities|Array|Get(acopy) _materials (Math|Random|RandomInteger (Utilities|Array|Length _materials)))))

(event Input|KeyboardEvents|F
  (params (Key :type Key%20Structure :default "AnyKey"))
  (:Released
    (Default|CallStamped (Utilities|Array|Get(acopy) (Actor|GetComponentsByClass (Variables|Default|GetSpawnedPerson) "/Game/Blueprints/Move.Move_C")))))

(fn ConstructionScript)