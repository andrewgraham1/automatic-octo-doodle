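; Movement component that walks its owning actor along world Y, holding it at a stop point until a stamp event arrives.
; Each Tick advances the owner with a swept move while short of StopLocation or while Continue is set.
; The Stamped event sets Continue and NewPerson clears it.
; When movement reaches FinalLocation, it tells the first SpawnPerson actor found to spawn a new person.
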(event Custom|Stamped_Event
  (Variables|Default|SetContinue true))

(event Custom|NewPerson_Event
  (Variables|Default|SetContinue false))

(event EventTick
  (params (DeltaSeconds :type Float%20%28single-precision%29))
  (bind _returnvalue (Components|GetOwner))
  (bind _speed (Variables|Default|GetSpeed))
  (bind _returnvalue_2 (Transformation|GetActorLocation _returnvalue))
  (bind _returnvalue_3 (* DeltaSeconds _speed))
  (bind _returnvalue_4 (Math|Vector|MakeVector 0.0 _returnvalue_3 0.0))
  (bind _returnvalue_5 (+ _returnvalue_4 _returnvalue_2))
  (bind _y (Math|Vector|BreakVector _returnvalue_5))
  (if (or (>= (Variables|Default|GetStop%20Location) _y) (Variables|Default|GetContinue))
    (Transformation|SetActorLocation _returnvalue _returnvalue_5 true false)
    (if (>= _y (Variables|Default|GetFinal%20Location))
      (bind _outactors (Actor|GetAllActorsOfClass "/Game/Blueprints/SpawnPerson.SpawnPerson_C"))
      (Default|CallSpawnNewPerson (Utilities|Array|Get(acopy) _outactors)))))

(event EventBeginPlay
  (EventDispatchers|BindEventtoStamped (delegate Custom|Stamped_Event))
  (EventDispatchers|BindEventtoNewPerson (delegate Custom|NewPerson_Event)))